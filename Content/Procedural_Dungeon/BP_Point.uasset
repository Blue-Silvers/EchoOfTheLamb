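; A collectible point that relocates between point rooms (BP_PointsRoom) in the procedural dungeon each time the player collects it.
; On BeginPlay it gathers all point rooms and moves to the first one's SpawnPoint.
; Overlap by BP_FirstPersonCharacter calls WinPointMessage on the player and moves the same actor to the next room, cycling through the list in order.
; A DoOnce guards the overlap and resets after each move.
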(event `self.ReceiveBeginPlay`
  (bind _outactors (`GameplayStatics.GetAllActorsOfClass` "/Game/Procedural_Dungeon/Room/Speedroom/PointsRooms/BP_PointsRoom.BP_PointsRoom_C"))
  (bind _output_get (set `self.spawnList` _outactors))
  (`self.K2_SetActorLocation` (`SceneComponent.K2_GetComponentLocation` (`/Game/Procedural_Dungeon/Room/Speedroom/PointsRooms/BP_PointsRoom.SpawnPoint` (`|GetArrayItem` _output_get))))
  (`self.UpdateSpawnOrder`))

(event `self.Collider.OnComponentBeginOverlap`
  (params (OverlappedComponent :type "PrimitiveComponent Object Reference") (OtherActor :type "Actor Object Reference") (OtherComp :type "PrimitiveComponent Object Reference") (OtherBodyIndex :type Integer) (bFromSweep :type Boolean) (SweepResult :type "HitResult Structure (by ref)"))
  (if (== (`GameplayStatics.GetObjectClass` OtherActor) "/Game/FirstPerson/Blueprints/Player/BP_FirstPersonCharacter.BP_FirstPersonCharacter_C")
    ;[0 0 0] Next pos
    (`/Engine/EditorBlueprintResources/StandardMacros.DoOnce` false :!label _label
      (:`Completed`
        (message `/Game/FirstPerson/Blueprints/Player/BPI_Player.WinPoint` OtherActor)
        (`self.K2_SetActorLocation` (`SceneComponent.K2_GetComponentLocation` (`/Game/Procedural_Dungeon/Room/Speedroom/PointsRooms/BP_PointsRoom.SpawnPoint` (`|GetArrayItem` (`self.spawnList`) (`self.spawnOrder`)))))
        (`self.UpdateSpawnOrder`)
        (`self.resetDoOnce`)))))

(event `resetDoOnce`
  (goto _label :!via `Reset`))

(fn `UpdateSpawnOrder`
  (bind _result (`/Engine/EditorBlueprintResources/StandardMacros.IncrementInt` (`self.spawnOrder`))
    (:`  `
      (if (>= _result (`KismetArrayLibrary.Array_Length` (`self.spawnList`)))
        (set `self.spawnOrder` 0)))))

(fn `UserConstructionScript`)