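; Procedural dungeon generator actor that builds a seeded random layout from a start room while showing a loading screen.
; Rooms attach at random open exits, retrying recursively on overlap and switching to the special room list for the final slots.
; Leftover exits get walls, then a map actor spawns from tracked room extents passed to GS_Main.
; A looping failsafe timer resets the saved seed and reloads the level if generation runs too long.
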(event `StartDungeonTimer`
  ;[0.3958 0 0] Generation Failsafe
  (bind _returnvalue (`KismetSystemLibrary.K2_SetTimerDelegate` (delegate `CheckForDungeonComplete`) 1.0 true))
  (set `self.timerHandle` _returnvalue))

(event `SetSeed`
  (bind _stream (`self.stream`))
  (bind _seed (`self.seed`))
  ;[0.4832 0 1] Set seed or generate random seed
  (if (== _seed -1)
    (`KismetMathLibrary.SeedRandomStream` _stream)
    (else
      (`KismetMathLibrary.SetRandomStreamSeed` _stream _seed)))
  (set `self.seed` (`KismetMathLibrary.BreakRandomStream` _stream)))

(event `CheckForDungeonComplete`
  (bind _asgi_main (cast `/Game/Manage/GI_Main` (`GameplayStatics.GetGameInstance`) :!pure true))
  ;[0.3958 0 0] Generation Failsafe
  (if (>= (`KismetSystemLibrary.GetGameTimeInSeconds`) (`self.maxDungeonTimeToLoad`))
    (bind _seed (`/Game/Manage/GI_Main.GetMaxPoint` _asgi_main))
    (`/Game/Manage/GI_Main.SaveSeed` _asgi_main -1 _seed)
    (bind _returnvalue (`GameplayStatics.GetCurrentLevelName` true))
    (`KismetSystemLibrary.ExecuteConsoleCommand` (`KismetStringLibrary.Concat_StrStr` "servertravel/Game/Maps/" _returnvalue "?listen") (`GameplayStatics.GetPlayerController` 0))))

(event `self.ReceiveBeginPlay`
  ;[0.05725 1 0] Start
  (`self.SetSeed`)
  (`self.SpawnStartRoom`)
  (`self.StartDungeonTimer`)
  (`self.SpawnNextRoom`)
  ;;[0 0.3594 1] LoadingScreen
  (`/Engine/EditorBlueprintResources/StandardMacros.IsValid` (`self.loadingRef`)
    (:`Is Valid`
      _)
    (:`Is Not Valid`
      (bind _returnvalue (`|CreateWidget` "/Game/UI/WBP_LoadingScreen.WBP_LoadingScreen_C"))
      (bind _output_get (set `self.loadingRef` _returnvalue))))
  (set `/Game/UI/WBP_LoadingScreen.nbRoom` (`self.roomAmount`) _output_get)
  (`UserWidget.AddToViewport` (`self.loadingRef`) 0))

(event `SpawnStartRoom`
  ;[0 0 0] Spawn Start Room
  (bind _returnvalue (`|SpawnActorFromClass` "/Game/Procedural_Dungeon/Room/Speedroom/BP_StartRoom.BP_StartRoom_C" (`SceneComponent.K2_GetComponentToWorld` (`self.DefaultSceneRoot`)) "AlwaysSpawn" "MultiplyWithRoot" null null))
  (`KismetArrayLibrary.Array_Append` (`self.exitList`) (`SceneComponent.GetChildrenComponents` (`/Game/Procedural_Dungeon/Room/BP_MasterRoom.Exits` _returnvalue) false)))

(event `SpawnNextRoom`
  (bind _exitlist (`self.exitList`))
  (bind _overlaplist (`self.overlapList`))
  (bind _loadingref (`self.loadingRef`))
  ;[0 0 0] Spawn other room
  (bind _output_get (set `self.selectedExitPoint` (`KismetArrayLibrary.Array_RandomFromStream` _exitlist (`self.stream`))))
  (`KismetArrayLibrary.Array_RemoveItem` _exitlist _output_get)
  (bind _returnvalue (`|SpawnActorFromClass` (`KismetArrayLibrary.Array_RandomFromStream` (`self.roomList`) (`self.stream`)) (`SceneComponent.K2_GetComponentToWorld` _output_get) "AlwaysSpawn" "MultiplyWithRoot" null null))
  (bind _asbp_master_room (cast `/Game/Procedural_Dungeon/Room/BP_MasterRoom` _returnvalue))
  (bind _output_get_2 (set `self.lastedRoom` _asbp_master_room))
  ;;[0 1 0.5249] Add Overlaping Room To List
  (for _array_element (`SceneComponent.GetChildrenComponents` (`/Game/Procedural_Dungeon/Room/BP_MasterRoom.OverlapFolder` _output_get_2) false)
    (bind _asprimitive_component (cast `PrimitiveComponent` _array_element))
    (`KismetArrayLibrary.Array_Append` (`self.overlapList`) (`PrimitiveComponent.GetOverlappingComponents` _asprimitive_component)))
  (if (`KismetArrayLibrary.Array_IsNotEmpty` _overlaplist)
    (`KismetArrayLibrary.Array_Clear` _overlaplist)
    (`self.K2_DestroyActor` (`self.lastedRoom`))
    (`KismetArrayLibrary.Array_Add` (`self.exitList`) (`self.selectedExitPoint`))
    (`self.SpawnNextRoom`)
    (else
      (`KismetArrayLibrary.Array_Clear` _overlaplist)
      (`self.SetMiddle of the map`)
      (`KismetArrayLibrary.Array_Append` (`self.exitList`) (`SceneComponent.GetChildrenComponents` (`/Game/Procedural_Dungeon/Room/BP_MasterRoom.Exits` (`self.lastedRoom`)) false))
      (bind _result (`/Engine/EditorBlueprintResources/StandardMacros.DecrementInt` (`self.roomAmount`))
        (:`  `
          ;;[0 0.3594 1] LoadingScreen
          (`/Engine/EditorBlueprintResources/StandardMacros.IsValid` _loadingref
            (:`Is Valid`
              (`/Game/UI/WBP_LoadingScreen.ChangeLoadingPercent` _loadingref (`self.roomAmount`)))
            (:`Is Not Valid`
              _))
          (if (> _result 0)
            (`KismetSystemLibrary.Delay` 0.1)
            (if (not (> (`self.roomAmount`) (`KismetArrayLibrary.Array_Length` (`self.specialRoomList`))))
              (`self.SetSpecialRoomSpawning`)
              (`KismetArrayLibrary.Array_RemoveItem` (`self.roomList`) (`GameplayStatics.GetObjectClass` (`self.lastedRoom`))))
            (`self.SpawnNextRoom`)
            (else
              (`self.CloseHoles`)
              (set `self.dungeonComplete` true)
              (`KismetSystemLibrary.K2_ClearAndInvalidateTimerHandle` (`self.timerHandle`))
              ;;[0 0.3594 1] LoadingScreen
              (`KismetSystemLibrary.Delay` 1.0)
              (`/Engine/EditorBlueprintResources/StandardMacros.IsValid` (`self.loadingRef`)
                (:`Is Valid`
                  (`Widget.RemoveFromParent` (`self.loadingRef`))
                  (`self.SpawnMap`))))))))))

(event `SetSpecialRoomSpawning`
  ;[0 0 0] Change room list
  (`/Engine/EditorBlueprintResources/StandardMacros.DoOnce` false
    (:`Completed`
      (set `self.roomList` (`self.specialRoomList`)))))

(event `CloseHoles`
  ;[0 0 0] Close holes
  (for _array_element (`self.exitList`)
    (`|SpawnActorFromClass` "/Game/Procedural_Dungeon/BP_CloseWall.BP_CloseWall_C" (`SceneComponent.K2_GetComponentToWorld` _array_element) "AlwaysSpawn" "MultiplyWithRoot" null null))
  (`|SpawnActorFromClass` "/Game/Procedural_Dungeon/BP_Point.BP_Point_C" (`SceneComponent.K2_GetComponentToWorld` (`self.DefaultSceneRoot`)) "Undefined" "MultiplyWithRoot" null null))

(event `SpawnMap`
  (bind _returnvalue (- (`self.minX`) (`self.maxX`)))
  (bind _returnvalue_2 (- (`self.minY`) (`self.maxY`)))
  ;[1 0 0] Map WIP
  ;;[1 0.965 0] Spawn cemera for map
  (`/Engine/EditorBlueprintResources/StandardMacros.DoOnce` false
    (:`Completed`
      (`|SpawnActorFromClass` "/Game/MapSystem/BP_Map.BP_Map_C" (`KismetMathLibrary.MakeTransform` (`KismetMathLibrary.MakeVector` (/ (+ (`self.maxX`) (`self.minX`)) 2.0) (/ (+ (`self.maxY`) (`self.minY`)) 2.0) 5000.0)) "Undefined" "MultiplyWithRoot" null null)
      (bind _asgs_main (cast `/Game/Manage/GS_Main` (`GameplayStatics.GetGameState`)))
      (set `/Game/Manage/GS_Main.Ortho Width` (+ (select `bool` (< _returnvalue _returnvalue_2) :`false` _returnvalue :`true` _returnvalue_2 :!type "Float (single-precision)") 15000.0) _asgs_main)
      (set `/Game/Manage/GS_Main.maxX` (`self.maxX`) _asgs_main)
      (set `/Game/Manage/GS_Main.minX` (`self.minX`) _asgs_main)
      (set `/Game/Manage/GS_Main.maxY` (`self.maxY`) _asgs_main)
      (set `/Game/Manage/GS_Main.minY` (`self.minY`) _asgs_main)
      (set `/Game/Manage/GS_Main.maxZ` (`self.maxZ`) _asgs_main)
      (set `/Game/Manage/GS_Main.minZ` (`self.minZ`) _asgs_main))))

(event `SetMiddle of the map`
  (bind (_returnvalue_x _returnvalue_y _returnvalue_z) (`KismetMathLibrary.BreakVector` (`self.K2_GetActorLocation` (`self.lastedRoom`))))
  (bind _returnvalue (> (`self.maxZ`) _returnvalue_z))
  (bind _returnvalue_2 (< (`self.minZ`) _returnvalue_z))
  (bind _returnvalue_3 (> (`self.maxX`) _returnvalue_x))
  (bind _returnvalue_4 (< (`self.minX`) _returnvalue_x))
  (bind _returnvalue_5 (> (`self.maxY`) _returnvalue_y))
  (bind _returnvalue_6 (< (`self.minY`) _returnvalue_y))
  ;[1 0 0] Map WIP
  ;;[1 0.965 0] Set pos for map
  (if (or _returnvalue_3 _returnvalue_4 _returnvalue_5 _returnvalue_6 _returnvalue _returnvalue_2)
    (if _returnvalue_3
      (set `self.maxX` _returnvalue_x))
    (if _returnvalue_4
      (set `self.minX` _returnvalue_x))
    (if _returnvalue_5
      (set `self.maxY` _returnvalue_y))
    (if _returnvalue_6
      (set `self.minY` _returnvalue_y))
    (if _returnvalue
      (set `self.maxZ` _returnvalue_z))
    (if _returnvalue_2
      (set `self.minZ` _returnvalue_z))))

(fn `UserConstructionScript`)