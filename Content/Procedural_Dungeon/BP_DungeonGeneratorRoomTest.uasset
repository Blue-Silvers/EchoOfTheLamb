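; BP_DungeonGeneratorRoomTest procedurally builds a dungeon at BeginPlay from a seeded random stream, behind a loading screen.
; Starting from BP_BasicRoom1, it attaches random rooms to open exits, destroying and retrying any that overlap.
; The final placements switch to the special room list, removing used classes, then walls cap leftover exits.
; A looping timer reloads the level if generation exceeds its time limit.
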(event `StartDungeonTimer`
  ;[0.3958 0 0] Generation Failsafe
  (bind _returnvalue (`KismetSystemLibrary.K2_SetTimerDelegate` (delegate `CheckForDungeonComplete`) 1.0 true))
  (set `self.timerHandle` _returnvalue))

(event `SetSeed`
  (bind _seed (`self.seed`))
  (bind _stream (`self.stream`))
  ;[0.4832 0 1] Set seed or generate random seed
  (if (== _seed -1)
    (`KismetMathLibrary.SeedRandomStream` _stream)
    (else
      (`KismetMathLibrary.SetRandomStreamSeed` _stream _seed)))
  (set `self.seed` (`KismetMathLibrary.BreakRandomStream` _stream)))

(event `CheckForDungeonComplete`
  ;[0.3958 0 0] Generation Failsafe
  (if (>= (`KismetSystemLibrary.GetGameTimeInSeconds`) (`self.maxDungeonTimeToLoad`))
    (bind _returnvalue (`GameplayStatics.GetCurrentLevelName` true))
    (`GameplayStatics.OpenLevel` (`KismetStringLibrary.Conv_StringToName` _returnvalue))))

(event `self.ReceiveBeginPlay`
  ;[0.05725 1 0] Start
  (`self.SetSeed`)
  (`self.SpawnStartRoom`)
  (`self.StartDungeonTimer`)
  (`self.SpawnNextRoom`)
  ;;[0 0.3594 1] LoadingScreen
  (`/Engine/EditorBlueprintResources/StandardMacros.IsValid` (`self.loadingRef`)
    (:`Is Valid`
      _)
    (:`Is Not Valid`
      (bind _returnvalue (`|CreateWidget` "/Game/UI/WBP_LoadingScreen.WBP_LoadingScreen_C"))
      (bind _output_get (set `self.loadingRef` _returnvalue))))
  (set `/Game/UI/WBP_LoadingScreen.nbRoom` (`self.roomAmount`) _output_get)
  (`UserWidget.AddToViewport` (`self.loadingRef`) 0))

(event `SpawnStartRoom`
  ;[0 0 0] Spawn Start Room
  (bind _returnvalue (`|SpawnActorFromClass` "/Game/Procedural_Dungeon/Room/BP_BasicRoom1.BP_BasicRoom1_C" (`SceneComponent.K2_GetComponentToWorld` (`self.DefaultSceneRoot`)) "AlwaysSpawn" "MultiplyWithRoot" null null))
  (`KismetArrayLibrary.Array_Append` (`self.exitList`) (`SceneComponent.GetChildrenComponents` (`/Game/Procedural_Dungeon/Room/BP_MasterRoom.Exits` _returnvalue) false)))

(event `SpawnNextRoom`
  (bind _exitlist (`self.exitList`))
  (bind _overlaplist (`self.overlapList`))
  (bind _loadingref (`self.loadingRef`))
  ;[0 0 0] Spawn other room
  (bind _output_get (set `self.selectedExitPoint` (`KismetArrayLibrary.Array_RandomFromStream` _exitlist (`self.stream`))))
  (`KismetArrayLibrary.Array_RemoveItem` _exitlist _output_get)
  (bind _returnvalue (`|SpawnActorFromClass` (`KismetArrayLibrary.Array_RandomFromStream` (`self.roomList`) (`self.stream`)) (`SceneComponent.K2_GetComponentToWorld` _output_get) "AlwaysSpawn" "MultiplyWithRoot" null null))
  (bind _asbp_master_room (cast `/Game/Procedural_Dungeon/Room/BP_MasterRoom` _returnvalue))
  (set `self.lastedRoom` _asbp_master_room)
  ;;[0 1 0.5249] Add Overlaping Room To List
  (`KismetArrayLibrary.Array_Append` (`self.overlapList`) (`PrimitiveComponent.GetOverlappingComponents` (`/Game/Procedural_Dungeon/Room/BP_MasterRoom.OverlapBox` (`self.lastedRoom`))))
  (if (`KismetArrayLibrary.Array_IsNotEmpty` _overlaplist)
    (`KismetArrayLibrary.Array_Clear` _overlaplist)
    (`self.K2_DestroyActor` (`self.lastedRoom`))
    (`KismetArrayLibrary.Array_Add` (`self.exitList`) (`self.selectedExitPoint`))
    (`self.SpawnNextRoom`)
    (else
      (`KismetArrayLibrary.Array_Clear` _overlaplist)
      (`KismetArrayLibrary.Array_Append` (`self.exitList`) (`SceneComponent.GetChildrenComponents` (`/Game/Procedural_Dungeon/Room/BP_MasterRoom.Exits` (`self.lastedRoom`)) false))
      (bind _result (`/Engine/EditorBlueprintResources/StandardMacros.DecrementInt` (`self.roomAmount`))
        (:`  `
          ;;[0 0.3594 1] LoadingScreen
          (`/Engine/EditorBlueprintResources/StandardMacros.IsValid` _loadingref
            (:`Is Valid`
              (`/Game/UI/WBP_LoadingScreen.ChangeLoadingPercent` _loadingref (`self.roomAmount`)))
            (:`Is Not Valid`
              _))
          (if (> _result 0)
            (`KismetSystemLibrary.Delay` 0.1)
            (if (not (> (`self.roomAmount`) (`KismetArrayLibrary.Array_Length` (`self.specialRoomList`))))
              (`self.SetSpecialRoomSpawning`)
              (`KismetArrayLibrary.Array_RemoveItem` (`self.roomList`) (`GameplayStatics.GetObjectClass` (`self.lastedRoom`))))
            (`self.SpawnNextRoom`)
            (else
              (`self.CloseHoles`)
              (set `self.dungeonComplete` true)
              (`KismetSystemLibrary.K2_ClearAndInvalidateTimerHandle` (`self.timerHandle`))
              ;;[0 0.3594 1] LoadingScreen
              (`KismetSystemLibrary.Delay` 1.0)
              (`/Engine/EditorBlueprintResources/StandardMacros.IsValid` (`self.loadingRef`)
                (:`Is Valid`
                  (`Widget.RemoveFromParent` (`self.loadingRef`)))))))))))

(event `SetSpecialRoomSpawning`
  ;[0 0 0] Change room list
  (`/Engine/EditorBlueprintResources/StandardMacros.DoOnce` false
    (:`Completed`
      (set `self.roomList` (`self.specialRoomList`)))))

(event `CloseHoles`
  ;[0 0 0] Close holes
  (for _array_element (`self.exitList`)
    (`|SpawnActorFromClass` "/Game/Procedural_Dungeon/BP_CloseWall.BP_CloseWall_C" (`SceneComponent.K2_GetComponentToWorld` _array_element) "AlwaysSpawn" "MultiplyWithRoot" null null)))

(fn `UserConstructionScript`)