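; BP_ItemRoom is an item room Blueprint for the procedural dungeon that provides a rifle pickup.
; On BeginPlay it runs the parent logic, waits through a short delay, then spawns BP_Pickup_Rifle at the SpawnPoint component's world transform.
; The pickup class is hard-coded, and the overlap and tick events are disabled.
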(event `self.ReceiveBeginPlay`
  (`parent.ReceiveBeginPlay`)
  (`KismetSystemLibrary.Delay` 2.0)
  (`|SpawnActorFromClass` "/Game/FirstPerson/Blueprints/Weapon/BP_Pickup_Rifle.BP_Pickup_Rifle_C" (`SceneComponent.K2_GetComponentToWorld` (`self.SpawnPoint`)) "Undefined" "MultiplyWithRoot" null null))

(fn `UserConstructionScript`
  (`parent.UserConstructionScript`))