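; BP_MasterRoom is a procedural dungeon room Blueprint that can hide its roof from the minimap's scene capture.
; The construction script tags the direct children of the RoofFolder component as "roof".
; BeginPlay gathers every primitive component with that tag into RoofList.
; SetRoofHiddenforMinimap runs once through a DoOnce and sets those components hidden in scene capture.
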(event `self.ReceiveBeginPlay`
  ;[0.4922 0 1] Listing roof element
  (for _array_element (`self.K2_GetComponentsByClass` "/Script/Engine.PrimitiveComponent")
    (if (`KismetArrayLibrary.Array_Contains` (`ActorComponent.ComponentTags` _array_element) "roof")
      (`KismetArrayLibrary.Array_Add` (`self.RoofList`) _array_element))))

(event `self.ReceiveActorBeginOverlap`
  (params (OtherActor :type "Actor Object Reference")))

(event `self.ReceiveTick`
  (params (DeltaSeconds :type "Float (single-precision)")))

(event `/Game/Procedural_Dungeon/BPI_Room.SetRoofHiddenForMinimap`
  ;[1 0.779 0] Desable roof for minimap
  (`/Engine/EditorBlueprintResources/StandardMacros.DoOnce` false
    (:`Completed`
      (for _array_element (`self.RoofList`)
        (`PrimitiveComponent.SetHiddenInSceneCapture` _array_element true)))))

(fn `UserConstructionScript`
  ;[1 0.1333 0.8566] Add roof tag for every component drop in Roof Folder
  (for _array_element (`SceneComponent.GetChildrenComponents` (`self.RoofFolder`) false)
    (`KismetArrayLibrary.Array_Add` (`ActorComponent.ComponentTags` _array_element) "roof")))