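; Map actor that moves an orthographic scene capture between top, right, left, front and back views of a bounded area.
; SwitchAngleOfView plays a timeline that lerps location and shortest-path rotation toward the view selected by SideView.
; Top restores the position and ortho width cached one tick after BeginPlay.
; Side views are offset from the Min/Max bounds, with ortho width set to the largest Min-minus-Max difference plus padding.
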(event `self.ReceiveBeginPlay`
  (`KismetSystemLibrary.DelayUntilNextTick`)
  (set `self.basePos` (`self.K2_GetActorLocation`))
  (set `self.Ortho Width` (`SceneCaptureComponent2D.OrthoWidth` (`self.SceneCaptureComponent2D`))))

(event `SwitchAngleOfView`
  (bind _returnvalue (/ (+ (`self.maxX`) (`self.minX`)) 2.0))
  (bind _returnvalue_2 (/ (+ (`self.maxY`) (`self.minY`)) 2.0))
  ;[1 0.8456 0] Switch angle of view
  (bind (_direction _alpha) (`Timeline|CameraTransition` :!via `PlayFromStart`)
    (:`Update`
      (switch `/Game/MapSystem/Enum_MapSide` (`self.SideView`)
        (:`NewEnumerator0`
          (`self.K2_SetActorLocationAndRotation` (`KismetMathLibrary.VLerp` (`self.K2_GetActorLocation`) (`self.basePos`) _alpha) (`KismetMathLibrary.RLerp` (`self.K2_GetActorRotation`) (struct) _alpha true)) ; Top
          (set `SceneCaptureComponent2D.OrthoWidth` (`self.Ortho Width`) (`self.SceneCaptureComponent2D`)))
        (:`NewEnumerator1`
          (`self.K2_SetActorLocationAndRotation` (`KismetMathLibrary.VLerp` (`self.K2_GetActorLocation`) (`KismetMathLibrary.MakeVector` _returnvalue (- (`self.minY`) -15000.0) (`self.ZMiddle`)) _alpha) (`KismetMathLibrary.RLerp` (`self.K2_GetActorRotation`) (`self.rightRotator`) _alpha true)) ; Right
          (`self.ChangeOrthoWightOtherSide`))
        (:`NewEnumerator2`
          (`self.K2_SetActorLocationAndRotation` (`KismetMathLibrary.VLerp` (`self.K2_GetActorLocation`) (`KismetMathLibrary.MakeVector` _returnvalue (+ (`self.maxY`) -15000.0) (`self.ZMiddle`)) _alpha) (`KismetMathLibrary.RLerp` (`self.K2_GetActorRotation`) (`self.leftRotation`) _alpha true)) ; Left
          (`self.ChangeOrthoWightOtherSide`))
        (:`NewEnumerator3`
          (`self.K2_SetActorLocationAndRotation` (`KismetMathLibrary.VLerp` (`self.K2_GetActorLocation`) (`KismetMathLibrary.MakeVector` (- (`self.minX`) -15000.0) _returnvalue_2 (`self.ZMiddle`)) _alpha) (`KismetMathLibrary.RLerp` (`self.K2_GetActorRotation`) (`self.frontRotation`) _alpha true)) ; Front
          (`self.ChangeOrthoWightOtherSide`))
        (:`NewEnumerator4`
          (`self.K2_SetActorLocationAndRotation` (`KismetMathLibrary.VLerp` (`self.K2_GetActorLocation`) (`KismetMathLibrary.MakeVector` (+ (`self.maxX`) -15000.0) _returnvalue_2 (`self.ZMiddle`)) _alpha) (`KismetMathLibrary.RLerp` (`self.K2_GetActorRotation`) (`self.backRotation`) _alpha true)) ; Back
          (`self.ChangeOrthoWightOtherSide`))))))

(fn `ChangeOrthoWightOtherSide`
  (bind _returnvalue (- (`self.minX`) (`self.maxX`)))
  (bind _returnvalue_2 (- (`self.minY`) (`self.maxY`)))
  (bind _returnvalue_3 (- (`self.minZ`) (`self.maxZ`)))
  (bind _returnvalue_4 (select `bool` (< _returnvalue _returnvalue_2) :`false` _returnvalue :`true` _returnvalue_2 :!type "Float (single-precision)"))
  (set `SceneCaptureComponent2D.OrthoWidth` (+ (select `bool` (< _returnvalue_3 _returnvalue_4) :`false` _returnvalue_3 :`true` _returnvalue_4 :!type "Float (single-precision)") 15000.0) (`self.SceneCaptureComponent2D`)))

(fn `UserConstructionScript`)