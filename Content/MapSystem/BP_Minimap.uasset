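; Minimap actor with a scene capture component whose near clipping plane adjusts to a Target actor.
; Each Tick, while Target is valid, it sets the second capture component's custom near plane to slightly less than the distance to Target, within a clamped range.
; An unconnected SetActorLocation node that would place the actor at a fixed height over Target never runs.
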(event `self.ReceiveTick`
  (params (DeltaSeconds :type "Float (single-precision)"))
  (bind _target (`self.Target`))
  (`/Engine/EditorBlueprintResources/StandardMacros.IsValid` _target
    (:`Is Valid`
      (set `SceneCaptureComponent2D.CustomNearClippingPlane` (`KismetMathLibrary.FClamp` (- (`KismetMathLibrary.Vector_Distance` (`self.K2_GetActorLocation` _target) (`self.K2_GetActorLocation`)) 500.0) 0.0 10000.0) (`self.SecondSceneCaptureComponent2D`)))))

(fn `UserConstructionScript`)