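; Lobby game mode that spawns joining players and tracks whether the match can start.
; On PostLogin it possesses a new BP_FirstPersonCharacter at a random PlayerStart, calls LoadGame on GI_Main and sets CanStartMatch.
; Player count checks against the PlayerArray gate launch-button HUD updates on login, and clearing CanStartMatch on logout.
; Login reaches the HUD through the first PC_Lobby, while logout uses the first player's character.
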(event `self.K2_PostLogin`
  (params (NewPlayer :type "PlayerController Object Reference"))
  ;[0 0 0] Player lunch game
  (bind _output_get (set `self.New Player` NewPlayer))
  ;;[0 0.39 0.4115] Spawn players
  (bind _outactors (`GameplayStatics.GetAllActorsOfClass` "/Script/Engine.PlayerStart"))
  (`WidgetBlueprintLibrary.SetInputMode_GameAndUIEx` _output_get null)
  (bind _returnvalue (`|SpawnActorFromClass` "/Game/FirstPerson/Blueprints/Player/BP_FirstPersonCharacter.BP_FirstPersonCharacter_C" (`self.GetTransform` (`KismetArrayLibrary.Array_Random` _outactors)) "Undefined" "MultiplyWithRoot" null _output_get null))
  (`Controller.Possess` _output_get _returnvalue)
  (bind _asgi_main (cast `/Game/Manage/GI_Main` (`GameplayStatics.GetGameInstance`)))
  (`/Game/Manage/GI_Main.LoadGame` _asgi_main)
  (set `self.canStartMatch` true)
  (`self.GetNumPlayers`)
  (bind _returnvalue_2 (`self.GetNumPlayers` (`GameplayStatics.GetGameMode`)))
  (if (>= _returnvalue_2 (`KismetArrayLibrary.Array_Length` (`GameStateBase.PlayerArray` (`GameplayStatics.GetGameState`))))
    (bind _aspc_lobby (cast `/Game/Manage/PC_Lobby` (`GameplayStatics.GetPlayerController` 0)))
    (bind _hud (`/Game/Manage/PC_Lobby.hud` _aspc_lobby))
    (`/Engine/EditorBlueprintResources/StandardMacros.IsValid` _hud
      (:`Is Valid`
        (`/Game/UI/WBP_HUD.LunchGameVisibility` _hud)))))

(event `self.K2_OnLogout`
  (params (ExitingController :type "Controller Object Reference"))
  ;[0 0 0] Player quit game
  (bind _returnvalue (`self.GetNumPlayers`))
  (if (< _returnvalue (`KismetArrayLibrary.Array_Length` (`GameStateBase.PlayerArray` (`GameplayStatics.GetGameState`))))
    (set `self.canStartMatch` false)
    (bind _asbp_first_person_character (cast `/Game/FirstPerson/Blueprints/Player/BP_FirstPersonCharacter` (`GameplayStatics.GetPlayerCharacter` 0)))
    (bind _hud (`/Game/FirstPerson/Blueprints/Player/BP_FirstPersonCharacter.hud` _asbp_first_person_character))
    (`/Engine/EditorBlueprintResources/StandardMacros.IsValid` _hud
      (:`Is Valid`
        (`/Game/UI/WBP_HUD.LunchGameVisibility` _hud)))))

(fn `UserConstructionScript`)