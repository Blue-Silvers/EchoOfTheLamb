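; Player controller for a match that shows the starting countdown and signals the game state when it has possessed a pawn.
; On BeginPlay, the local controller hides the cursor and adds the WBP_StartingMatch countdown widget to the viewport.
; Possession chains through OnPossessClient to ClientIsPossess, which sets IsPossess and calls LunchGame on GS_Main.
; ShowCountDown updates the widget, retrying every tick until it is valid.
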(event `self.ReceiveBeginPlay`
  (if (`self.IsLocalPlayerController`)
    (set `self.bShowMouseCursor` false)
    (bind _returnvalue (`|CreateWidget` "/Game/UI/WBP_StartingMatch.WBP_StartingMatch_C" self))
    (bind _output_get (set `self.Countdown` _returnvalue))
    (`UserWidget.AddToViewport` _output_get 0)))

(event `ShowCountDown`
  (bind _countdown (`self.Countdown`))
  (`/Engine/EditorBlueprintResources/StandardMacros.IsValid` _countdown :!label _label
    (:`Is Valid`
      (`/Game/UI/WBP_StartingMatch.CountDownUpdate` _countdown))
    (:`Is Not Valid`
      (`KismetSystemLibrary.DelayUntilNextTick`)
      (goto _label))))

(event `self.ReceivePossess`
  (params (PossessedPawn :type "Pawn Object Reference"))
  (`self.OnPossessClient`))

(event `OnPossessClient`
  (`self.ClientIsPossess`))

(event `ClientIsPossess`
  (set `self.isPossess` true)
  (`/Game/Manage/GS_Main.LunchGame` (cast `/Game/Manage/GS_Main` (`GameplayStatics.GetGameState`) :!pure true)))

(fn `UserConstructionScript`)