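; GM_Match is the match game mode that sets up players and the procedural dungeon.
; On each login it spawns and possesses a first-person character at a random PlayerStart, then loads the saved game through GI_Main.
; A DoOnce then spawns the dungeon generator with the game instance's seed, records that seed, and copies the win point target from GI_Main into GS_Main.
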(event `self.K2_PostLogin`
  (params (NewPlayer :type "PlayerController Object Reference"))
  ;[0 0 0] Post login
  ;;[0 0.39 0.4115] Spawn players
  (bind _outactors (`GameplayStatics.GetAllActorsOfClass` "/Script/Engine.PlayerStart"))
  (`WidgetBlueprintLibrary.SetInputMode_GameOnly` NewPlayer)
  (bind _returnvalue (`|SpawnActorFromClass` "/Game/FirstPerson/Blueprints/Player/BP_FirstPersonCharacter.BP_FirstPersonCharacter_C" (`self.GetTransform` (`KismetArrayLibrary.Array_Random` _outactors)) "Undefined" "MultiplyWithRoot" null NewPlayer null))
  (bind _output_get (set `self.newPlayer` _returnvalue))
  (`Controller.Possess` NewPlayer _output_get)
  (bind _asgi_main (cast `/Game/Manage/GI_Main` (`GameplayStatics.GetGameInstance`)))
  (`/Game/Manage/GI_Main.LoadGame` _asgi_main)
  ;[0 0 0] Spawn Dungeon
  (`/Engine/EditorBlueprintResources/StandardMacros.DoOnce` false
    (:`Completed`
      (bind _seed (`/Game/Manage/GI_Main.GetSeed` _asgi_main))
      (bind _returnvalue_2 (`|SpawnActorFromClass` "/Game/Procedural_Dungeon/BP_DungeaonGenerator.BP_DungeaonGenerator_C" (`self.spawnDungon`) "Undefined" "MultiplyWithRoot" null 25 _seed null))
      (set `self.dungeon` _returnvalue_2)
      (`self.UpdateSeed` _seed)
      (bind _seed_2 (`/Game/Manage/GI_Main.GetMaxPoint` _asgi_main))
      (bind _output_get_2 (set `self.maxPointsForWin` _seed_2))
      (set `/Game/Manage/GS_Main.maxPointsForWin` _output_get_2 (cast `/Game/Manage/GS_Main` (`GameplayStatics.GetGameState`) :!pure true)))))

(event `UpdateSeed`
  (params (Seed :type Integer))
  (if (== (`self.seedGM`) -1)
    (set `self.seedGM` Seed)))

(fn `UserConstructionScript`)