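; GM_Main is the game mode that spawns joining players and tracks whether the match can start.
; PostLogin spawns a BP_ThirdPersonCharacter at a random PlayerStart, loads GI_Main's save and sets CanStartMatch, even below the minimum player count.
; Reaching that minimum, or dropping below it on logout, calls LunchGameVisibility on the first player's HUD; dropping below also clears the flag.
; Unwired LAN session nodes never run.
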(event `self.K2_PostLogin`
  (params (NewPlayer :type "PlayerController Object Reference"))
  ;[0 0 0] Player lunch game
  (bind _output_get (set `self.New Player` NewPlayer))
  ;;[0 0.39 0.4115] Spawn players
  (bind _outactors (`GameplayStatics.GetAllActorsOfClass` "/Script/Engine.PlayerStart"))
  (`|SpawnActorFromClass` "/Game/ThirdPerson/Blueprints/BP_ThirdPersonCharacter.BP_ThirdPersonCharacter_C" (`self.GetTransform` (`KismetArrayLibrary.Array_Random` _outactors)) "Undefined" "MultiplyWithRoot" null _output_get null)
  (bind _asgi_main (cast `/Game/Manage/GI_Main` (`GameplayStatics.GetGameInstance`)))
  (`/Game/Manage/GI_Main.LoadGame` _asgi_main)
  (set `self.canStartMatch` true)
  (bind _returnvalue (`self.GetNumPlayers`))
  (if (>= _returnvalue (`self.MinNumberOfPlayer`))
    (bind _aspc_main (cast `/Game/Manage/PC_Main` (`GameplayStatics.GetPlayerController` 0)))
    (bind _hud (`/Game/Manage/PC_Main.hud` _aspc_main))
    (`/Engine/EditorBlueprintResources/StandardMacros.IsValid` _hud
      (:`Is Valid`
        (`/Game/UI/WBP_HUD.LunchGameVisibility` _hud)))))

(event `self.K2_OnLogout`
  (params (ExitingController :type "Controller Object Reference"))
  ;[0 0 0] Player quit game
  (bind _returnvalue (`self.GetNumPlayers`))
  (if (< _returnvalue (`self.MinNumberOfPlayer`))
    (set `self.canStartMatch` false)
    (bind _asbp_third_person_character (cast `/Game/ThirdPerson/Blueprints/BP_ThirdPersonCharacter` (`GameplayStatics.GetPlayerCharacter` 0)))
    (bind _hud (`/Game/ThirdPerson/Blueprints/BP_ThirdPersonCharacter.hud` _asbp_third_person_character))
    (`/Engine/EditorBlueprintResources/StandardMacros.IsValid` _hud
      (:`Is Valid`
        (`/Game/UI/WBP_HUD.LunchGameVisibility` _hud)))))

(fn `UserConstructionScript`)